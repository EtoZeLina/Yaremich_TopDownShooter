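; BP_Spider1 is a spider enemy that chases and attacks the player.
; A looping AIMoveTo pursues the player, while Tick plays an attack montage in range, pausing movement until it completes.
; DamagePlayer applies range-checked damage but has no caller here.
; Incoming damage sets HP to clamped damage minus HP; at zero, the spider deactivates, increments BP_Soldier_01's kills and is destroyed after a delay.
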(event EventBeginPlay
  ;[1 1 1] AI MOVE
  (if (CallFunction|IsAlive) :!label _label
    (AI|AIMoveTo self "0, 0, 0" (Game|GetPlayerCharacter 0) 5.0 false
      (:OnSuccess
        _)
      (:OnFail
        _))
    (Utilities|FlowControl|Delay 0.2)
    (goto _label)))

(event EventTick
  (params (DeltaSeconds :type Float%20%28single-precision%29))
  ;[1 1 1] Attack
  (if (Math|Boolean|ANDBoolean (CallFunction|IsAttackRange) (not (CallFunction|IsAttacking)) (CallFunction|IsAlive))
    (Components|Activation|Deactivate (Variables|Character|GetCharacterMovement))
    (Animation|Montage|PlayMontage (Variables|Character|GetMesh) "/Game/Characters/Enemy_Great_Spider/Animations/SpiderAttack_01.SpiderAttack_01"
      (:OnCompleted
        (Components|Activation|Activate (Variables|Character|GetCharacterMovement) false)))))

(event Game|Damage|EventAnyDamage
  (params (Damage :type Float%20%28single-precision%29) (DamageType :type Damage%20Type%20Object%20Reference) (InstigatedBy :type Controller%20Object%20Reference) (DamageCauser :type Actor%20Object%20Reference))
  ;[1 1 1] HP
  (bind _output_get (CallFunction|DecreaseHP Damage))
  (if (== _output_get 0.0)
    (CallFunction|SpiderDeactivate)
    (Utilities|FlowControl|Delay 5.0)
    (Actor|DestroyActor)))

(fn ConstructionScript)

(fn IsAttackRange
  (return (>= (LocalVariables|GetAttackRange) (Transformation|GetDistanceTo (Game|GetPlayerCharacter 0)))))

(fn IsAttacking
  (return (Animation|Montage|MontageIsPlaying (Components|SkeletalMesh|GetAnimInstance (Variables|Character|GetMesh)) "/Game/Characters/Enemy_Great_Spider/Animations/SpiderAttack_01.SpiderAttack_01")))

(fn DamagePlayer
  (if (CallFunction|IsAttackRange)
    (Game|Damage|ApplyDamage (Game|GetPlayerCharacter 0) (LocalVariables|Getdamage%20pre%20hit) 0 0)))

(fn DecreaseHP
  (params (Damage :type Float%20%28single-precision%29))
  (bind _output_get (Variables|Default|SetSpider_HP (Math|Float|Clamp(Float) (- Damage (Variables|Default|GetSpider_HP)) 0.0 1e+02)))
  (return _output_get))

(fn SpiderDeactivate
  (Variables|Default|SetIs_Dead true)
  (Components|Activation|Deactivate (Variables|Character|GetCharacterMovement))
  (Collision|SetActorEnableCollision false)
  (Components|Movement|StopMovementImmediately (Variables|Character|GetCharacterMovement))
  (CallFunction|IncreaseKills)
  (return))

(fn IsAlive
  (return (not (Variables|Default|GetIs_Dead))))

(fn IncreaseKills
  (bind _asbp_soldier_01 (Utilities|Casting|CastToBP_Soldier_01 (Game|GetPlayerCharacter 0)))
  (Math|Integer|IncrementInt (Variables|/Game/Blueprints/Actors/BP_Soldier_01.BP_Soldier_01_C|GetKills _asbp_soldier_01)))